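; Game mode Blueprint that handles the main menu flow: showing the menu, starting a new game and quitting.
; MainMenu disables player input, displays WBP_MainMenu and binds to its new game and exit click dispatchers.
; StartNewGame restores input, removes the widget and opens TheLevel, while ExitGame quits.
; BeginPlay is empty and the graph's own MainMenu call is disconnected, so nothing here triggers the menu.
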(event Custom|MainMenu
  (Input|DisableInput (Game|GetPlayerController 0) 0)
  (bind _returnvalue (UserInterface|CreateWidget "/Game/Blueprints/UMG/WBP_MainMenu.WBP_MainMenu_C"))
  (bind _output_get (Variables|Default|SetWidget_MainMenu _returnvalue))
  (UserInterface|Viewport|AddtoViewport _output_get 0)
  (EventDispatchers|BindEventtoOnStartNewGameClicked _output_get (EventDispatchers|CreateEvent :!event Custom|StartNewGame))
  (EventDispatchers|BindEventtoOnExitClicked _output_get (EventDispatchers|CreateEvent :!event Custom|ExitGame)))

(event Custom|StartNewGame
  (Input|EnableInput (Game|GetPlayerController 0) 0)
  (Widget|RemovefromParent (Variables|Default|GetWidget_MainMenu))
  (Game|OpenLevel(byName) "TheLevel" true "Start"))

(event Custom|ExitGame
  (Game|QuitGame 0 "Quit" false))

(event EventBeginPlay)

(fn ConstructionScript)