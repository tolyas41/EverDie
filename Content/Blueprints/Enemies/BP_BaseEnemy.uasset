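; Base Paper2D enemy that tracks health, plays an attack animation and is destroyed at zero HP.
; An AttackRadius overlap with BP_EverDiePlayer signals attack readiness, and BeginPlay passes the attack animation length out as an AI parameter.
; AttackAction swaps to the attack flipbook, then back to movement after a retriggerable delay.
; Damage updates the HP bar widget and triggers Death when health runs out.
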(event OnComponentBeginOverlap(AttackRadius)
  (params (OverlappedComponent :type Primitive%20Component%20Object%20Reference) (OtherActor :type Actor%20Object%20Reference) (OtherComp :type Primitive%20Component%20Object%20Reference) (OtherBodyIndex :type Integer) (bFromSweep :type Boolean) (SweepResult :type Hit%20Result%20Structure%20%28by%20ref%29))
  (Utilities|Casting|CastToBP_EverDiePlayer OtherActor)
  (Default|CallReadyAttack))

(event OnComponentEndOverlap(AttackRadius)
  (params (OverlappedComponent :type Primitive%20Component%20Object%20Reference) (OtherActor :type Actor%20Object%20Reference) (OtherComp :type Primitive%20Component%20Object%20Reference) (OtherBodyIndex :type Integer))
  (Utilities|Casting|CastToBP_EverDiePlayer OtherActor)
  (Default|CallNotReadyAttack))

(event Custom|AttackAction
  (Sprite|SetFlipbook (Variables|Default|GetPaperFlipbook) (Variables|Default|GetAttackAnim))
  (Utilities|FlowControl|RetriggerableDelay (Variables|Default|GetAttackAnimLength))
  (Sprite|SetFlipbook (Variables|Default|GetPaperFlipbook) (Variables|Default|GetMoveAnim)))

(event Custom|Death
  (Actor|DestroyActor))

(event EventBeginPlay
  (bind _output_get (Variables|Default|SetAttackAnimLength (Class|PaperFlipbook|GetTotalDuration (Variables|Default|GetAttackAnim))))
  (Default|CallSetAIParams _output_get)
  (bind _aswbp_enemy_hp (Utilities|Casting|CastToWBP_EnemyHP (UserInterface|GetWidget (Variables|Default|GetHPBar))))
  (Variables|Default|SetWidgetHPBar _aswbp_enemy_hp)
  (Variables|Default|SetHP (Variables|Default|GetMaxHP)))

(event EventDamage
  (params (Damage :type Float%20%28single-precision%29))
  (bind _output_get (Variables|Default|SetHP (- (Variables|Default|GetHP) Damage)))
  (Default|SetHPPercent (Variables|Default|GetWidgetHPBar) (/ _output_get (Variables|Default|GetMaxHP)))
  (if (<= _output_get 0.0)
    (CallFunction|Death)))

(fn ConstructionScript)