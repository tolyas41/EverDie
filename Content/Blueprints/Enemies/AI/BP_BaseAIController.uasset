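; Base AI controller for enemies that runs the BT_Reaper behavior tree against the EverDie player.
; On BeginPlay it stores the player in the Blackboard as PlayerTarget and binds to the controlled BP_BaseEnemy's attack-readiness and AI-parameter events.
; Handlers write the AttackMode and AttackRate Blackboard keys, while the Attack event forwards to the pawn's AttackAction.
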(event Custom|SetAttackMode
  (AI|Components|Blackboard|SetValueasBool (Variables|Default|GetBlackboard) (Utilities|Name|MakeLiteralName "AttackMode") true))

(event Custom|SetNonAttackMode
  (AI|Components|Blackboard|SetValueasBool (Variables|Default|GetBlackboard) (Utilities|Name|MakeLiteralName "AttackMode") false))

(event Custom|Attack
  (Default|AttackAction (Variables|Default|GetControlledPawn)))

(event EventBeginPlay
  (bind _returnvalue (Actor|GetActorOfClass "/Game/Blueprints/Player/BP_EverDiePlayer.BP_EverDiePlayer_C"))
  (Variables|Default|SetPlayerTarget _returnvalue)
  (AI|RunBehaviorTree "/Game/Blueprints/Enemies/Reaper/AI/BT_Reaper.BT_Reaper")
  (AI|Components|Blackboard|SetValueasObject (Variables|Default|GetBlackboard) (Utilities|Name|MakeLiteralName "PlayerTarget") (Variables|Default|GetPlayerTarget))
  (bind _asbp_base_enemy (Utilities|Casting|CastToBP_BaseEnemy (Pawn|GetControlledPawn)))
  (bind _output_get (Variables|Default|SetControlledPawn _asbp_base_enemy))
  (EventDispatchers|BindEventtoReadyAttack _output_get (EventDispatchers|CreateEvent :!event Custom|SetAttackMode))
  (EventDispatchers|BindEventtoNotReadyAttack _output_get (EventDispatchers|CreateEvent :!event Custom|SetNonAttackMode))
  (EventDispatchers|BindEventtoSetAIParams _output_get (EventDispatchers|CreateEvent :!event UpdateBB)))

(fn ConstructionScript)

(fn UpdateBB
  (params (AttackRate :type Float%20%28single-precision%29))
  (AI|Components|Blackboard|SetValueasFloat (Variables|Default|GetBlackboard) (Utilities|Name|MakeLiteralName "AttackRate") AttackRate))