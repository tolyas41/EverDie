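; Enemy manager that repeatedly spawns BP_ReaperEnemy actors during play.
; After a short startup delay it caches the BP_EverDiePlayer reference and starts a looping timer at SpawnRate.
; Each tick of the timer spawns a reaper at the location from GetRandomPointInRadiusAroundPlayer.
; That function holds only unconnected math for signed random X and Z offsets between SpawnRadiusMin and SpawnRadiusMax from the player.
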(event Custom|SpawnEnemy
  (Game|SpawnActorfromClass "/Game/Blueprints/Enemies/Reaper/BP_ReaperEnemy.BP_ReaperEnemy_C" (Math|Transform|MakeTransform (Utilities|GetRandomPointinRadiusAroundPlayer) "0, 0, 0" "1,1,1") "Undefined" 0 "3.000000,3.000000,3.000000" 0))

(event EventBeginPlay
  (Utilities|FlowControl|Delay 0.2)
  (bind _returnvalue (Actor|GetActorOfClass "/Game/Blueprints/Player/BP_EverDiePlayer.BP_EverDiePlayer_C"))
  (Variables|Default|SetPlayerRef _returnvalue)
  (bind _returnvalue_2 (Utilities|Time|SetTimerbyEvent (delegate Custom|SpawnEnemy) (Variables|Default|GetSpawnRate) true))
  (Variables|Default|SetTH_Spawner _returnvalue_2))

(fn ConstructionScript)