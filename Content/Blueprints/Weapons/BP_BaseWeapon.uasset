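; Base weapon pickup that fires projectiles toward a cursor location for the EverDie player.
; Capsule overlap with the player sets it as the equipped weapon, attaches it, hides its sprite and copies its directional idle, move and attack animations onto the character.
; Attack spawns the projectile class aimed at the cursor, with a one-shot timer at AttackRate acting as a cooldown; the timer's AutoAttack event is empty.
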(event OnComponentBeginOverlap(Capsule)
  (params (OverlappedComponent :type Primitive%20Component%20Object%20Reference) (OtherActor :type Actor%20Object%20Reference) (OtherComp :type Primitive%20Component%20Object%20Reference) (OtherBodyIndex :type Integer) (bFromSweep :type Boolean) (SweepResult :type Hit%20Result%20Structure%20%28by%20ref%29))
  (bind _self self)
  (bind _asbp_ever_die_player (Utilities|Casting|CastToBP_EverDiePlayer OtherActor))
  (Variables|/Game/Blueprints/Player/BP_EverDiePlayer.BP_EverDiePlayer_C|SetEquippedWeapon _asbp_ever_die_player _self)
  (Transformation|AttachActorToActor _self _asbp_ever_die_player "None" "SnapToTarget" "SnapToTarget" "SnapToTarget" true)
  (Rendering|SetVisibility (Variables|Default|GetSprite _self) false false)
  (CallFunction|SetCharAnimations _asbp_ever_die_player))

(event Custom|Attack
  (params (CursorLocation :type Vector))
  (bind _returnvalue (Transformation|GetActorLocation))
  (bind _returnvalue_2 (Math|Rotator|FindLookatRotation _returnvalue CursorLocation))
  (if (not (Utilities|Time|IsTimerActivebyHandle (Variables|Default|GetAutoAttackTH)))
    (bind _returnvalue_3 (Utilities|Time|SetTimerbyEvent (delegate Custom|AutoAttack) (Variables|Default|GetAttackRate)))
    (Variables|Default|SetAutoAttackTH _returnvalue_3)
    (Game|SpawnActorfromClass (Variables|Default|GetProjectileClass) (Math|Transform|MakeTransform _returnvalue _returnvalue_2 "1,1,1") "Undefined" 0 _returnvalue_2 0)))

(event Custom|AutoAttack)

(fn ConstructionScript)

(fn SetCharAnimations
  (params (Char :type BP%20Ever%20Die%20Player%20Object%20Reference))
  ;[1 1 1 0] :)
  (Variables|/Game/Blueprints/Player/BP_EverDiePlayer.BP_EverDiePlayer_C|SetAnimAttackDown Char (Variables|Animation|GetAnimAttackDown))
  (Variables|/Game/Blueprints/Player/BP_EverDiePlayer.BP_EverDiePlayer_C|SetAnimAttackLeft Char (Variables|Animation|GetAnimAttackLeft))
  (Variables|/Game/Blueprints/Player/BP_EverDiePlayer.BP_EverDiePlayer_C|SetAnimAttackRight Char (Variables|Animation|GetAnimAttackRight))
  (Variables|/Game/Blueprints/Player/BP_EverDiePlayer.BP_EverDiePlayer_C|SetAnimAttackUp Char (Variables|Animation|GetAnimAttackUp))
  (Variables|/Game/Blueprints/Player/BP_EverDiePlayer.BP_EverDiePlayer_C|SetAnimIdleDown Char (Variables|Animation|GetAnimIdleDown))
  (Variables|/Game/Blueprints/Player/BP_EverDiePlayer.BP_EverDiePlayer_C|SetAnimIdleLeft Char (Variables|Animation|GetAnimIdleLeft))
  (Variables|/Game/Blueprints/Player/BP_EverDiePlayer.BP_EverDiePlayer_C|SetAnimIdleRight Char (Variables|Animation|GetAnimIdleRight))
  (Variables|/Game/Blueprints/Player/BP_EverDiePlayer.BP_EverDiePlayer_C|SetAnimIdleUp Char (Variables|Animation|GetAnimIdleUp))
  (Variables|/Game/Blueprints/Player/BP_EverDiePlayer.BP_EverDiePlayer_C|SetAnimMoveDown Char (Variables|Animation|GetAnimMoveDown))
  (Variables|/Game/Blueprints/Player/BP_EverDiePlayer.BP_EverDiePlayer_C|SetAnimMoveLeft Char (Variables|Animation|GetAnimMoveLeft))
  (Variables|/Game/Blueprints/Player/BP_EverDiePlayer.BP_EverDiePlayer_C|SetAnimMoveRight Char (Variables|Animation|GetAnimMoveRight))
  (Variables|/Game/Blueprints/Player/BP_EverDiePlayer.BP_EverDiePlayer_C|SetAnimMoveUp Char (Variables|Animation|GetAnimMoveUp)))