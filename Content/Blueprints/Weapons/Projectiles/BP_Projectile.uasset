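; Projectile actor with a Paper2D sprite that damages enemies on overlap.
; The construction script copies ProjectileSpeed into the ProjectileMovement initial speed, and BeginPlay zeroes the sprite's world roll and yaw while keeping its pitch.
; When the collision sphere overlaps an actor implementing BI_EnemyDamage, it sends Damage through ReceiveDamageMessage and destroys itself, ignoring other actors.
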(event OnComponentBeginOverlap(SphereCollision)
  (params (OverlappedComponent :type Primitive%20Component%20Object%20Reference) (OtherActor :type Actor%20Object%20Reference) (OtherComp :type Primitive%20Component%20Object%20Reference) (OtherBodyIndex :type Integer) (bFromSweep :type Boolean) (SweepResult :type Hit%20Result%20Structure%20%28by%20ref%29))
  (if (Utilities|DoesObjectImplementInterface OtherActor "/Game/Blueprints/Enemies/BI_EnemyDamage.BI_EnemyDamage_C")
    (Class|BIEnemyDamage|ReceiveDamage(Message) OtherActor (Variables|Default|GetDamage))
    (Actor|DestroyActor)))

(event EventBeginPlay
  (bind _papersprite (Variables|Default|GetPaperSprite))
  (Transformation|SetWorldRotation _papersprite (Math|Rotator|MakeRotator 0.0 (.pitch (Transformation|GetWorldRotation _papersprite)) 0.0) false false))

(event Collision|EventActorBeginOverlap
  (params (OtherActor :type Actor%20Object%20Reference)))

(fn ConstructionScript
  (Variables|/Script/Engine.ProjectileMovementComponent|SetInitialSpeed (Variables|Default|GetProjectileMovement) (Variables|Default|GetProjectileSpeed)))