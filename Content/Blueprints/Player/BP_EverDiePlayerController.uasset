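; Player controller for EverDie that relays attack and animation requests to the player pawn and its equipped weapon.
; It caches the controlled BP_EverDiePlayer on BeginPlay.
; AttackAction passes its direction as a string to the pawn's move/idle animation switch, then triggers Attack, while SwitchIdleAnim passes an empty string.
; Attack aims the equipped weapon, if valid, at the world-static hit location under the cursor.
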(event Custom|Attack
  (bind _everdieplayerref (Variables|Default|GetEverDiePlayerRef))
  (bind _equippedweapon (Variables|/Game/Blueprints/Player/BP_EverDiePlayer.BP_EverDiePlayer_C|GetEquippedWeapon _everdieplayerref))
  (Utilities|IsValid _equippedweapon
    (:Is%20Valid
      (Default|Attack _equippedweapon (.Location (Collision|BreakHitResult (.HitResult (Class|PlayerController|GetHitResultUnderCursorforObjects (Utilities|Array|MakeArray (Utilities|Enum|LiteralenumEObjectTypeQuery "ObjectTypeQuery1")) true))))))))

(event EventBeginPlay
  (bind _asbp_ever_die_player (Utilities|Casting|CastToBP_EverDiePlayer (Pawn|GetControlledPawn)))
  (Variables|Default|SetEverDiePlayerRef _asbp_ever_die_player))

(event EventSwitchIdleAnim
  (Default|SwitchMoveIdleAnim (Variables|Default|GetEverDiePlayerRef)))

(event EventAttackAction
  (params (direction :type CharDirections%20Enum :default "Left"))
  (Default|SwitchMoveIdleAnim (Variables|Default|GetEverDiePlayerRef) (Utilities|String|EnumtoString direction))
  (CallFunction|Attack))

(fn ConstructionScript)